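; Side-scrolling sprite enemy that moves along the Y axis, chasing the player at close range and otherwise wandering left or right at random.
; Each Tick, downward traces check grounding and reverse wandering at drops, while the sprite flips with movement direction.
; When grounded, a fan of forward traces at rising heights detects where an obstacle ends and randomly triggers LaunchCharacter to jump, with all traces debug-drawn.
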(event `self.ReceiveBeginPlay`)

(event `self.ReceiveTick`
  (params (DeltaSeconds :type "Float (single-precision)"))
  (bind _charactermovement (`self.CharacterMovement`))
  (set `self.Distance_to_lpayer` (`KismetMathLibrary.Vector_Distance` (`self.K2_GetActorLocation`) (`self.K2_GetActorLocation` (`GameplayStatics.GetPlayerCharacter` 0))))
  (`self.Grounded_raycast`)
  (`self.Sprite_scale`)
  (`self.Raycast`)
  (`self.Jumping`)
  (`|ExecutionSequence`
    (:`then_0`
      (if (`self.Jump?`)
        _
        (elif (<= (`self.Distance_to_lpayer`) 250.0)
          (set `MovementComponent.Velocity` (+ (* (`KismetMathLibrary.Normal` (`KismetMathLibrary.GetDirectionUnitVector` (`self.K2_GetActorLocation`) (`self.K2_GetActorLocation` (`GameplayStatics.GetPlayerCharacter` 0)))) (0.0 250.0 0.0)) (0.0 0.0 -500.0)) _charactermovement)
          (else
            (set `MovementComponent.Velocity` (`self.Random_velocity`) _charactermovement)))))
    (:`then_1`
      (`KismetSystemLibrary.Delay` (`KismetMathLibrary.RandomFloatInRange` 0.5 2.0))
      (`self.Set velocity`))))

(event `Sprite_scale`
  (bind _sprite (`self.Sprite`))
  (bind (_returnvalue_x _returnvalue_y _returnvalue_z) (`KismetMathLibrary.BreakVector` (`SceneComponent.K2_GetComponentScale` _sprite)))
  (bind (_velocity_x _velocity_y) (`KismetMathLibrary.BreakVector` (`MovementComponent.Velocity` (`self.CharacterMovement`))))
  (if (< _velocity_y 0.0)
    (`/Engine/EditorBlueprintResources/StandardMacros.DoOnce` false :!label _label
      (:`Completed`
        (`SceneComponent.SetWorldScale3D` _sprite (`KismetMathLibrary.MakeVector` (* _returnvalue_x -1.0) _returnvalue_y _returnvalue_z))
        (goto _label_2 :!via `Reset`)))
    (else
      (`/Engine/EditorBlueprintResources/StandardMacros.DoOnce` false :!label _label_2
        (:`Completed`
          (`SceneComponent.SetWorldScale3D` _sprite (`KismetMathLibrary.MakeVector` (`KismetMathLibrary.Abs` _returnvalue_x) _returnvalue_y _returnvalue_z))
          (goto _label :!via `Reset`))))))

(event `Set velocity`
  (if (<= (`KismetMathLibrary.RandomIntegerInRange` 0 1) 0)
    (set `self.Random_velocity` (0.0 250.0 -500.0))
    (else
      (set `self.Random_velocity` (0.0 -250.0 -500.0)))))

(event `Raycast`
  (bind _returnvalue (`self.K2_GetActorLocation`))
  (bind (_random_velocity_x _random_velocity_y) (`KismetMathLibrary.BreakVector` (`self.Random_velocity`)))
  (bind (_outhit _returnvalue_2) (`KismetSystemLibrary.LineTraceSingle` :`Start` _returnvalue :`End` (- _returnvalue (0.0 0.0 500.0)) :`TraceChannel` "TraceTypeQuery1" :`DrawDebugType` "ForDuration" :`TraceColor` (struct :`R` 1.0 :`G` 0.911 :`B` 0.941491 :`A` 1.0) :`DrawTime` 0.1))
  (if (not _returnvalue_2)
    (set `self.Random_velocity` (`KismetMathLibrary.MakeVector` 0.0 (* _random_velocity_y -1.0) -500.0))))

(event `Grounded_raycast`
  (bind _returnvalue (`self.K2_GetActorLocation`))
  (bind (_outhit _returnvalue_2) (`KismetSystemLibrary.LineTraceSingle` :`Start` _returnvalue :`End` (- _returnvalue (0.0 0.0 100.0)) :`TraceChannel` "TraceTypeQuery1" :`DrawDebugType` "ForDuration" :`TraceColor` (struct :`R` 1.0 :`B` 0.956905 :`A` 1.0) :`TraceHitColor` (struct :`G` 0.045144 :`B` 1.0 :`A` 1.0) :`DrawTime` 0.1))
  (if _returnvalue_2
    (set `self.Grounded?` true)
    (else
      (set `self.Grounded?` false))))

(event `Jumping`
  (bind (_returnvalue_x _returnvalue_y _returnvalue_z) (`KismetMathLibrary.BreakVector` (`self.K2_GetActorLocation`)))
  (bind _returnvalue (`self.K2_GetActorLocation`))
  (bind (_returnvalue_x_2 _returnvalue_y_2 _returnvalue_z_2) (`KismetMathLibrary.BreakVector` (`self.K2_GetActorLocation`)))
  (bind (_last_hit_x _last_hit_y _last_hit_z) (`KismetMathLibrary.BreakVector` (`self.Last_hit`)))
  (bind (_returnvalue_x_3 _returnvalue_y_3) (`KismetMathLibrary.BreakVector` (`KismetMathLibrary.Normal` (`MovementComponent.Velocity` (`self.CharacterMovement`)))))
  (bind (_returnvalue_x_4 _returnvalue_y_4 _returnvalue_z_3) (`KismetMathLibrary.BreakVector` (`KismetMathLibrary.Normal` (`KismetMathLibrary.GetDirectionUnitVector` (`self.K2_GetActorLocation`) (`self.Last_hit`)))))
  (if (`self.Grounded?`)
    (if (not (`self.Jump?`))
      (set `self.Raycast_start` _returnvalue)
      (for _index (range 31)
        (bind (_outhit _returnvalue_2) (`KismetSystemLibrary.LineTraceSingle` :`Start` _returnvalue :`End` (+ (`KismetMathLibrary.MakeVector` _returnvalue_x _returnvalue_y _returnvalue_z) (`KismetMathLibrary.MakeVector` 0.0 (* _returnvalue_y_3 500.0) (* _index 15))) :`TraceChannel` "TraceTypeQuery1" :`DrawDebugType` "ForDuration" :`TraceColor` (struct :`R` 1.0 :`G` 0.911 :`B` 0.941491 :`A` 1.0) :`DrawTime` 0.1))
        (set `self.Last_hit` (`.Location` (`GameplayStatics.BreakHitResult` _outhit)))
        (`|ExecutionSequence`
          (:`then_0`
            (if _returnvalue_2
              (`/Engine/EditorBlueprintResources/StandardMacros.DoOnce` false :!label _label_3
                (:`Completed`
                  (set `self.First_ray_hit?` true)))))
          (:`then_1`
            (if _returnvalue_2
              _
              (elif (`self.First_ray_hit?`)
                (if (<= (`KismetMathLibrary.RandomIntegerInRange` 0 100) 25)
                  (set `self.Jump?` true)
                  (`self.LaunchCharacter` (`KismetMathLibrary.MakeVector` 0.0 (* _returnvalue_y_4 (* (- _last_hit_y _returnvalue_y_2) 2.0)) (`KismetMathLibrary.Abs` (* _returnvalue_z_3 (* (- _returnvalue_z_2 _last_hit_z) 4.0)))))
                  (`KismetSystemLibrary.Delay` 0.1)
                  (set `self.Jump?` false)))))))
      (set `self.First_ray_hit?` false)
      (goto _label_3 :!via `Reset`))))

(event `self.OnLanded`
  (params (Hit :type "HitResult Structure (by ref)"))
  (set `self.Grounded?` true)
  (if (`self.Jump?`)
    (set `self.Jump?` false)))

(fn `UserConstructionScript`)