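; Plant actor that grows from a seed sprite each time an overlapping actor tagged Rain touches it.
; Each hit advances the sprite list without a bounds check and adds audio, varying by growth stage with a rare random variant.
; A timeline enlarges the plant while a temporary sprite drifts and is destroyed by a second timeline.
; DoOnce gates block further hits until the scale timeline finishes and saves the new base scale.
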(event `self.ReceiveBeginPlay`
  (set `self.Base_scale` (`SceneComponent.K2_GetComponentScale` (`self.Graine_2-removebg-preview_Sprite`)))
  (`PaperSpriteComponent.SetSprite` (`self.Graine_2-removebg-preview_Sprite`) (`|GetArrayItem` (`self.List_sprite`))))

(event `self.Graine_2-removebg-preview_Sprite.OnComponentBeginOverlap`
  (params (OverlappedComponent :type "PrimitiveComponent Object Reference") (OtherActor :type "Actor Object Reference") (OtherComp :type "PrimitiveComponent Object Reference") (OtherBodyIndex :type Integer) (bFromSweep :type Boolean) (SweepResult :type "HitResult Structure (by ref)"))
  (bind _base_scale (`self.Base_scale`))
  (if (`self.ActorHasTag` OtherActor "Rain")
    (`/Engine/EditorBlueprintResources/StandardMacros.DoOnce` false :!label _label
      (:`Completed`
        (`/Engine/EditorBlueprintResources/StandardMacros.IncrementInt` (`self.Index_list_sprite`)
          (:`  `
            (`PaperSpriteComponent.SetSprite` (`self.Graine_2-removebg-preview_Sprite`) (`|GetArrayItem` (`self.List_sprite`) (`self.Index_list_sprite`)))
            (if (== (`KismetMathLibrary.RandomIntegerInRange` 0 100) 100)
              (`AddComponent|NODE_AddAudioComponent-2`)
              (`KismetSystemLibrary.PrintString` "MEEEEEEEEEEEOOOOOOOOOOOOWWWWWWWWWWWW")
              (bind (_direction _newtrack_0) (`Timeline|Timeline_0` :!via `PlayFromStart` :!label _label_2)
                (:`Update`
                  (`SceneComponent.SetWorldScale3D` (`self.Graine_2-removebg-preview_Sprite`) (`KismetMathLibrary.VLerp` _base_scale (+ _base_scale (0.1 0.1 0.1)) _newtrack_0))
                  (`/Engine/EditorBlueprintResources/StandardMacros.DoOnce` false :!label _label_3
                    (:`Completed`
                      (bind _returnvalue (`AddComponent|NODE_AddPaperSpriteComponent-0` :`RelativeTransform` (`KismetMathLibrary.MakeTransform` (`self.K2_GetActorLocation`) (struct :`Yaw` 180.0) (0.05 0.05 0.05))))
                      (bind (_direction_2 _newtrack_1) (`Timeline|Timeline_1` :!via `PlayFromStart`)
                        (:`Update`
                          (bind _returnvalue_2 (`SceneComponent.K2_GetComponentLocation` _returnvalue))
                          (bind (_returnvalue_x _returnvalue_y _returnvalue_z) (`KismetMathLibrary.BreakVector` (`KismetMathLibrary.VLerp` _returnvalue_2 (+ _returnvalue_2 (0.0 0.0 1.0)) _newtrack_1)))
                          (`SceneComponent.K2_SetWorldLocation` _returnvalue (`KismetMathLibrary.MakeVector` 0.0 _returnvalue_y _returnvalue_z) false false))
                        (:`Finished`
                          (`ActorComponent.K2_DestroyComponent` _returnvalue))))))
                (:`Finished`
                  (`|ExecutionSequence`
                    (:`then_0`
                      (set `self.Base_scale` (`SceneComponent.K2_GetComponentScale` (`self.Graine_2-removebg-preview_Sprite`)))
                      (goto _label :!via `Reset`))
                    (:`then_1`
                      (goto _label_3 :!via `Reset`)))))
              (elif (>= (`self.Index_list_sprite`) 5)
                (`AddComponent|NODE_AddAudioComponent-1`)
                (`KismetSystemLibrary.PrintString` "aRA ARA")
                (goto _label_2 :!via `PlayFromStart`)
                (else
                  (`AddComponent|NODE_AddAudioComponent-0`)
                  (`KismetSystemLibrary.PrintString` "UwU")
                  (goto _label_2 :!via `PlayFromStart`))))))))))

(fn `UserConstructionScript`)