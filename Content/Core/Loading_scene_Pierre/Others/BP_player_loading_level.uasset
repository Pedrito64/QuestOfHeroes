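; Player character for the loading level, a sprite that moves left and right and hops while shedding rain drops.
; Jump input applies a small upward launch, rate-limited by a DoOnce and Delay, and timelines briefly narrow the sprite and restore it.
; While falling, Tick spawns rain drop actors below it after random delays.
; The FOV kick is disconnected, and the widget created on BeginPlay is never added to the viewport.
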(event `self.ReceiveBeginPlay`
  (bind (_returnvalue_x _returnvalue_y _returnvalue_z) (`KismetMathLibrary.BreakVector` (`SceneComponent.K2_GetComponentScale` (`self.Sprite`))))
  (bind (_returnvalue_x_2 _returnvalue_y_2) (`KismetMathLibrary.BreakVector` (/ (`KismetMathLibrary.MakeVector` _returnvalue_x _returnvalue_y _returnvalue_z) (`KismetMathLibrary.Conv_DoubleToVector` 1.35))))
  (set `self.Base_fov` 0.0)
  (set `self.New_fov` (- 0.0 5.0))
  (set `self.Base_scale` (`KismetMathLibrary.MakeVector` _returnvalue_x _returnvalue_y _returnvalue_z))
  (set `self.New_scale` (`KismetMathLibrary.MakeVector` _returnvalue_x_2 _returnvalue_y_2 _returnvalue_z))
  (bind _returnvalue (`|CreateWidget` "/Game/Core/Loading_scene_Pierre/Others/NewWidgetBlueprint.NewWidgetBlueprint_C"))
  (set `self.NewVar_0` _returnvalue))

(event `InputAction|Jump`
  (params (Key :type "Key Structure"))
  (:`Pressed`
    (`/Engine/EditorBlueprintResources/StandardMacros.DoOnce` false :!label _label
      (:`Completed`
        (`self.Jump_FOV`)
        (`self.Jump_scale`)
        (`self.LaunchCharacter` (0.0 0.0 150.0) false true)
        (`KismetSystemLibrary.Delay` 0.3)
        (goto _label :!via `Reset`)))))

(event `Jump_FOV`)

(event `Jump_scale`
  (bind _sprite (`self.Sprite`))
  (bind (_direction _newtrack_0) (`Timeline|Timeline_2` :`NewTime` 0.15 :!via `PlayFromStart`)
    (:`Update`
      (`SceneComponent.SetWorldScale3D` _sprite (`KismetMathLibrary.VLerp` (`self.Base_scale`) (`self.New_scale`) _newtrack_0)))
    (:`Finished`
      (bind (_direction_2 _newtrack_0_2) (`Timeline|Timeline_3` :`NewTime` 0.15 :!via `ReverseFromEnd`)
        (:`Update`
          (`SceneComponent.SetWorldScale3D` _sprite (`KismetMathLibrary.VLerp` (`self.Base_scale`) (`self.New_scale`) _newtrack_0_2)))))))

(event `InputAxis|Move Right / Left`
  (params (AxisValue :type "Float (single-precision)"))
  (`self.AddMovementInput` (`self.GetActorRightVector`) AxisValue))

(event `self.ReceiveTick`
  (params (DeltaSeconds :type "Float (single-precision)"))
  (if (`NavMovementComponent.IsFalling` (`self.CharacterMovement`))
    (`KismetSystemLibrary.Delay` (`KismetMathLibrary.RandomFloatInRange` 0.1 0.4))
    (`|SpawnActorFromClass` "/Game/Core/Loading_scene_Pierre/Others/BP_rain_drop.BP_rain_drop_C" (`KismetMathLibrary.MakeTransform` (- (`self.K2_GetActorLocation`) (`KismetMathLibrary.MakeVector` 0.0 (`KismetMathLibrary.RandomFloatInRange` 20.0 -20.0) 50.0)) (struct) (0.5 0.5 0.5)) "AlwaysSpawn" "OverrideRootScale" null null)))

(fn `UserConstructionScript`)