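; Procedural level manager that builds random runs of 2D sprite platforms in the Y-Z plane, starting at the origin on BeginPlay.
; Edge and corner events chain into each other randomly, advancing a shared spawn cursor with direction flags until an iteration cap.
; Top and bottom runs roll rare enemy spawns, ignoring the ChanceToSpawn input.
; Reset_tick resets the counter and restarts generation from a random point based on player location.
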(event `Spawn_enemy`
  (params (Spawn_location :type "Vector Structure") (`Chance to spawn` :type Integer))
  (if (<= (`KismetMathLibrary.RandomIntegerInRange` 0 100) 0)
    (`|SpawnActorFromClass` "/Game/Core/Loading_scene_Pierre/BP_enemy.BP_enemy_C" (`KismetMathLibrary.MakeTransform` Spawn_location (struct :`Yaw` 90.0) (0.5 0.5 0.5)) "AdjustIfPossibleButAlwaysSpawn" "OverrideRootScale" null null)))

(event `Set number iteration`
  (set `self.Current_number_iterations` (+ (`self.Current_number_iterations`) 1))
  (if (>= (`self.Current_number_iterations`) (`self.Max_number_iterations`))
    (set `self.Stop?` true)))

(event `self.ReceiveBeginPlay`
  (set `self.Spawn Transform Location` (0.0 0.0 0.0))
  (`self.Bot_generation` :!label _label))

(event `Reset_tick`
  (bind _returnvalue (`self.K2_GetActorLocation` (`GameplayStatics.GetPlayerCharacter` 0)))
  (set `self.Current_number_iterations` 0)
  (set `self.Max_number_iterations` 10)
  (set `self.Stop?` false)
  (set `self.Spawn Transform Location` (`KismetMathLibrary.RandomPointInBoundingBox` _returnvalue (+ _returnvalue (0.0 250.0 250.0))))
  (goto _label))

(event `Bot_generation`
  (bind _returnvalue (`KismetMathLibrary.RandomIntegerInRange` 4 50))
  (bind (_spawn_transform_location_x _spawn_transform_location_y _spawn_transform_location_z) (`KismetMathLibrary.BreakVector` (`self.Spawn Transform Location`)))
  (if (not (`self.Stop?`))
    (`self.Set number iteration`)
    ;[1 1 1] BOTTOM GENERATION
    (for _index (range (+ _returnvalue 1))
      (bind _returnvalue_2 (* _index 15))
      (bind _returnvalue_3 (`KismetMathLibrary.SelectFloat` (+ _spawn_transform_location_y _returnvalue_2) (- _spawn_transform_location_y _returnvalue_2) (`self.Select_right`)))
      (bind _returnvalue_4 (`|SpawnActorFromClass` "/Game/Core/Loading_scene_Pierre/BP_platform.BP_platform_C" (`KismetMathLibrary.MakeTransform` (`KismetMathLibrary.MakeVector` _spawn_transform_location_x _returnvalue_3 _spawn_transform_location_z)) "AlwaysSpawn" "OverrideRootScale" null null))
      (`self.Spawn_enemy` (`KismetMathLibrary.MakeVector` _spawn_transform_location_x _returnvalue_3 (+ _spawn_transform_location_z 30.0)) _returnvalue)
      (`PaperSpriteComponent.SetSprite` (`/Game/Core/Loading_scene_Pierre/BP_platform.Sprite` _returnvalue_4) (`KismetArrayLibrary.Array_Random` (`self.List_of_bot_sprites`))))
    (bind _output_get (set `self.Spawn Transform Location` (`KismetMathLibrary.MakeVector` _spawn_transform_location_x _returnvalue_3 _spawn_transform_location_z)))
    (`self.Spawn_enemy` _output_get)
    (if (== (`KismetMathLibrary.RandomIntegerInRange` 0 1) 0)
      (`self.Bot_right_generation`)
      (else
        (`self.Bot_left_generation`)))))

(event `Bot_left_generation`
  (bind (_spawn_transform_location_x _spawn_transform_location_y _spawn_transform_location_z) (`KismetMathLibrary.BreakVector` (`self.Spawn Transform Location`)))
  ;[1 1 1] BOT LEFT GENERATION
  (if (not (`self.Stop?`))
    (`self.Set number iteration`)
    (bind _returnvalue (`|SpawnActorFromClass` "/Game/Core/Loading_scene_Pierre/BP_platform.BP_platform_C" (`KismetMathLibrary.MakeTransform` (`KismetMathLibrary.MakeVector` _spawn_transform_location_x _spawn_transform_location_y _spawn_transform_location_z)) "AlwaysSpawn" "OverrideRootScale" null null))
    (`PaperSpriteComponent.SetSprite` (`/Game/Core/Loading_scene_Pierre/BP_platform.Sprite` _returnvalue) (`KismetArrayLibrary.Array_Random` (`self.List_of_bot_left_sprites`)))
    (set `self.Spawn Transform Location` (`KismetMathLibrary.MakeVector` _spawn_transform_location_x _spawn_transform_location_y (- _spawn_transform_location_z 15.0)))
    (if (== (`KismetMathLibrary.RandomIntegerInRange` 0 1) 0)
      (set `self.Select_down` true)
      (`self.Left_generation`)
      (else
        (set `self.Select_right` true)
        (`self.Bot_generation`)))))

(event `Top_generation`
  (bind _returnvalue (`KismetMathLibrary.RandomIntegerInRange` 4 50))
  (bind (_spawn_transform_location_x _spawn_transform_location_y _spawn_transform_location_z) (`KismetMathLibrary.BreakVector` (`self.Spawn Transform Location`)))
  (if (not (`self.Stop?`))
    (`self.Set number iteration`)
    ;[1 1 1] TOP GENERATION
    (for _index (range (+ _returnvalue 1))
      (bind _returnvalue_2 (* _index 15))
      (bind _returnvalue_3 (+ _spawn_transform_location_y _returnvalue_2))
      (bind _returnvalue_4 (`KismetMathLibrary.SelectFloat` _returnvalue_3 (- _spawn_transform_location_y _returnvalue_2) (`self.Select_right`)))
      (bind _returnvalue_5 (`|SpawnActorFromClass` "/Game/Core/Loading_scene_Pierre/BP_platform.BP_platform_C" (`KismetMathLibrary.MakeTransform` (`KismetMathLibrary.MakeVector` _spawn_transform_location_x _returnvalue_3 _returnvalue_4)) "AlwaysSpawn" "OverrideRootScale" null null))
      (`self.Spawn_enemy` (`KismetMathLibrary.MakeVector` _spawn_transform_location_x _returnvalue_4 (+ _spawn_transform_location_z 30.0)) _returnvalue)
      (`PaperSpriteComponent.SetSprite` (`/Game/Core/Loading_scene_Pierre/BP_platform.Sprite` _returnvalue_5) (`KismetArrayLibrary.Array_Random` (`self.List_of_top_right_sprites`))))
    (set `self.Spawn Transform Location` (`KismetMathLibrary.MakeVector` _spawn_transform_location_x _returnvalue_4 _spawn_transform_location_z))
    (if (== (`KismetMathLibrary.RandomIntegerInRange` 0 1) 0)
      (`self.Top_right_generation`)
      (else
        (`self.Top_left_generation`)))))

(event `Bot_right_generation`
  (bind (_spawn_transform_location_x _spawn_transform_location_y _spawn_transform_location_z) (`KismetMathLibrary.BreakVector` (`self.Spawn Transform Location`)))
  ;[1 1 1] BOT RIGHT GENERATION
  (if (not (`self.Stop?`))
    (`self.Set number iteration`)
    (bind _returnvalue (`|SpawnActorFromClass` "/Game/Core/Loading_scene_Pierre/BP_platform.BP_platform_C" (`KismetMathLibrary.MakeTransform` (`KismetMathLibrary.MakeVector` _spawn_transform_location_x _spawn_transform_location_y _spawn_transform_location_z)) "AlwaysSpawn" "OverrideRootScale" null null))
    (`PaperSpriteComponent.SetSprite` (`/Game/Core/Loading_scene_Pierre/BP_platform.Sprite` _returnvalue) (`KismetArrayLibrary.Array_Random` (`self.List_of_bot_right_sprites`)))
    (set `self.Spawn Transform Location` (`KismetMathLibrary.MakeVector` _spawn_transform_location_x _spawn_transform_location_y (+ _spawn_transform_location_z 15.0)))
    (if (== (`KismetMathLibrary.RandomIntegerInRange` 0 1) 0)
      (set `self.Select_down` false)
      (`self.Right_generation`)
      (else
        (set `self.Select_right` false)
        (`self.Bot_generation`)))))

(event `Left_generation`
  (bind (_spawn_transform_location_x _spawn_transform_location_y _spawn_transform_location_z) (`KismetMathLibrary.BreakVector` (`self.Spawn Transform Location`)))
  ;[1 1 1] LEFT GENERATION
  (if (not (`self.Stop?`))
    (`self.Set number iteration`)
    (for _index (range (+ (`KismetMathLibrary.RandomIntegerInRange` 2 25) 1))
      (bind _returnvalue (* _index 15))
      (bind _returnvalue_2 (`KismetMathLibrary.SelectFloat` (- _spawn_transform_location_z _returnvalue) (+ _spawn_transform_location_z _returnvalue) (`self.Select_down`)))
      (bind _returnvalue_3 (`|SpawnActorFromClass` "/Game/Core/Loading_scene_Pierre/BP_platform.BP_platform_C" (`KismetMathLibrary.MakeTransform` (`KismetMathLibrary.MakeVector` _spawn_transform_location_x _spawn_transform_location_y _returnvalue_2)) "AlwaysSpawn" "OverrideRootScale" null null))
      (`PaperSpriteComponent.SetSprite` (`/Game/Core/Loading_scene_Pierre/BP_platform.Sprite` _returnvalue_3) (`KismetArrayLibrary.Array_Random` (`self.List_of_left_sprites`))))
    (set `self.Spawn Transform Location` (`KismetMathLibrary.MakeVector` _spawn_transform_location_x _spawn_transform_location_y _returnvalue_2))
    (if (== (`KismetMathLibrary.RandomIntegerInRange` 0 1) 0)
      (`self.Bot_left_generation`)
      (else
        (`self.Top_left_generation`)))))

(event `Top_left_generation`
  (bind (_spawn_transform_location_x _spawn_transform_location_y _spawn_transform_location_z) (`KismetMathLibrary.BreakVector` (`self.Spawn Transform Location`)))
  ;[1 1 1] TOP LEFT GENERATION
  (if (not (`self.Stop?`))
    (`self.Set number iteration`)
    (bind _returnvalue (`|SpawnActorFromClass` "/Game/Core/Loading_scene_Pierre/BP_platform.BP_platform_C" (`KismetMathLibrary.MakeTransform` (`KismetMathLibrary.MakeVector` _spawn_transform_location_x _spawn_transform_location_y _spawn_transform_location_z)) "AlwaysSpawn" "OverrideRootScale" null null))
    (`PaperSpriteComponent.SetSprite` (`/Game/Core/Loading_scene_Pierre/BP_platform.Sprite` _returnvalue) (`KismetArrayLibrary.Array_Random` (`self.List_of_top_left_sprites`)))
    (set `self.Spawn Transform Location` (`KismetMathLibrary.MakeVector` _spawn_transform_location_x _spawn_transform_location_y (+ _spawn_transform_location_z 15.0)))
    (if (== (`KismetMathLibrary.RandomIntegerInRange` 0 1) 0)
      (set `self.Select_down` true)
      (`self.Left_generation`)
      (else
        (set `self.Select_right` true)
        (`self.Top_generation`)))))

(event `Right_generation`
  (bind (_spawn_transform_location_x _spawn_transform_location_y _spawn_transform_location_z) (`KismetMathLibrary.BreakVector` (`self.Spawn Transform Location`)))
  ;[1 1 1] RIGHT GENERATION
  (if (not (`self.Stop?`))
    (`self.Set number iteration`)
    (for _index (range (+ (`KismetMathLibrary.RandomIntegerInRange` 2 25) 1))
      (bind _returnvalue (* _index 15))
      (bind _returnvalue_2 (`KismetMathLibrary.SelectFloat` (- _spawn_transform_location_z _returnvalue) (+ _spawn_transform_location_z _returnvalue) (`self.Select_down`)))
      (bind _returnvalue_3 (`|SpawnActorFromClass` "/Game/Core/Loading_scene_Pierre/BP_platform.BP_platform_C" (`KismetMathLibrary.MakeTransform` (`KismetMathLibrary.MakeVector` _spawn_transform_location_x _spawn_transform_location_y _returnvalue_2)) "AlwaysSpawn" "OverrideRootScale" null null))
      (`PaperSpriteComponent.SetSprite` (`/Game/Core/Loading_scene_Pierre/BP_platform.Sprite` _returnvalue_3) (`KismetArrayLibrary.Array_Random` (`self.List_of_right_sprites`))))
    (set `self.Spawn Transform Location` (`KismetMathLibrary.MakeVector` _spawn_transform_location_x _spawn_transform_location_y _returnvalue_2))
    (if (== (`KismetMathLibrary.RandomIntegerInRange` 0 1) 0)
      (`self.Bot_right_generation`)
      (else
        (`self.Top_right_generation`)))))

(event `Top_right_generation`
  (bind (_spawn_transform_location_x _spawn_transform_location_y _spawn_transform_location_z) (`KismetMathLibrary.BreakVector` (`self.Spawn Transform Location`)))
  ;[1 1 1] TOP RIGHT GENERATION
  (if (not (`self.Stop?`))
    (`self.Set number iteration`)
    (bind _returnvalue (`|SpawnActorFromClass` "/Game/Core/Loading_scene_Pierre/BP_platform.BP_platform_C" (`KismetMathLibrary.MakeTransform` (`KismetMathLibrary.MakeVector` _spawn_transform_location_x _spawn_transform_location_y _spawn_transform_location_z)) "AlwaysSpawn" "OverrideRootScale" null null))
    (`PaperSpriteComponent.SetSprite` (`/Game/Core/Loading_scene_Pierre/BP_platform.Sprite` _returnvalue) (`KismetArrayLibrary.Array_Random` (`self.List_of_top_right_sprites`)))
    (set `self.Spawn Transform Location` (`KismetMathLibrary.MakeVector` _spawn_transform_location_x _spawn_transform_location_y (+ _spawn_transform_location_z 15.0)))
    (if (== (`KismetMathLibrary.RandomIntegerInRange` 0 1) 0)
      (set `self.Select_right` false)
      (`self.Top_generation`)
      (else
        (set `self.Select_down` true)
        (`self.Right_generation`)))))

(fn `Get random item in list`
  (params (Array :type "Array of PaperSprite Object Reference") (TargetArray :type "Array of PaperSprite Object Reference (by ref)"))
  (returns (Output :type "PaperSprite Object Reference"))
  (return (`|GetArrayItem` Array (`KismetMathLibrary.RandomIntegerInRange` 0 (`KismetArrayLibrary.Array_LastIndex` TargetArray)))))

(fn `UserConstructionScript`)