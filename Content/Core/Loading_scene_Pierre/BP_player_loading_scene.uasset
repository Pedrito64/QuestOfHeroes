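; Player character for a loading scene that moves left and right, hops with visual feedback and drips rain drops while airborne.
; Jump is gated by a DoOnce with a short delay, launches the character upward and triggers forward-then-reverse timelines that narrow camera FOV and shrink the sprite in X and Y.
; While falling, Tick uses a random Delay to space out small BP_rain_drop spawns below it with random sideways offset.
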(event `self.ReceiveBeginPlay`
  (bind (_returnvalue_x _returnvalue_y _returnvalue_z) (`KismetMathLibrary.BreakVector` (`SceneComponent.K2_GetComponentScale` (`self.Sprite`))))
  (bind _fieldofview (`CameraComponent.FieldOfView` (`self.Camera`)))
  (bind (_returnvalue_x_2 _returnvalue_y_2) (`KismetMathLibrary.BreakVector` (/ (`KismetMathLibrary.MakeVector` _returnvalue_x _returnvalue_y _returnvalue_z) (`KismetMathLibrary.Conv_DoubleToVector` 1.35))))
  (set `self.Base_fov` _fieldofview)
  (set `self.New_fov` (- _fieldofview 5.0))
  (set `self.Base_scale` (`KismetMathLibrary.MakeVector` _returnvalue_x _returnvalue_y _returnvalue_z))
  (set `self.New_scale` (`KismetMathLibrary.MakeVector` _returnvalue_x_2 _returnvalue_y_2 _returnvalue_z)))

(event `InputAction|Jump`
  (params (Key :type "Key Structure"))
  (:`Pressed`
    (`/Engine/EditorBlueprintResources/StandardMacros.DoOnce` false :!label _label
      (:`Completed`
        (`self.Jump_FOV`)
        (`self.Jump_scale`)
        (`self.LaunchCharacter` (0.0 0.0 150.0) false true)
        (`KismetSystemLibrary.Delay` 0.3)
        (goto _label :!via `Reset`)))))

(event `Jump_FOV`
  (bind _camera (`self.Camera`))
  (bind (_direction _newtrack_0) (`Timeline|Timeline_0` :`NewTime` 0.15 :!via `PlayFromStart`)
    (:`Update`
      (`CameraComponent.SetFieldOfView` _camera (`KismetMathLibrary.Lerp` (`self.Base_fov`) (`self.New_fov`) _newtrack_0)))
    (:`Finished`
      (bind (_direction_2 _newtrack_0_2) (`Timeline|Timeline_1` :`NewTime` 0.15 :!via `ReverseFromEnd`)
        (:`Update`
          (`CameraComponent.SetFieldOfView` _camera (`KismetMathLibrary.Lerp` (`self.Base_fov`) (`self.New_fov`) _newtrack_0_2)))))))

(event `Jump_scale`
  (bind _sprite (`self.Sprite`))
  (bind (_direction _newtrack_0) (`Timeline|Timeline_2` :`NewTime` 0.15 :!via `PlayFromStart`)
    (:`Update`
      (`SceneComponent.SetWorldScale3D` _sprite (`KismetMathLibrary.VLerp` (`self.Base_scale`) (`self.New_scale`) _newtrack_0)))
    (:`Finished`
      (bind (_direction_2 _newtrack_0_2) (`Timeline|Timeline_3` :`NewTime` 0.15 :!via `ReverseFromEnd`)
        (:`Update`
          (`SceneComponent.SetWorldScale3D` _sprite (`KismetMathLibrary.VLerp` (`self.Base_scale`) (`self.New_scale`) _newtrack_0_2)))))))

(event `InputAxis|Move Right / Left`
  (params (AxisValue :type "Float (single-precision)"))
  (`self.AddMovementInput` (`self.GetActorRightVector`) AxisValue))

(event `self.ReceiveTick`
  (params (DeltaSeconds :type "Float (single-precision)"))
  (if (`NavMovementComponent.IsFalling` (`self.CharacterMovement`))
    (`KismetSystemLibrary.Delay` (`KismetMathLibrary.RandomFloatInRange` 0.1 0.4))
    (`|SpawnActorFromClass` "/Game/Core/Loading_scene_Pierre/BP_rain_drop.BP_rain_drop_C" (`KismetMathLibrary.MakeTransform` (- (`self.K2_GetActorLocation`) (`KismetMathLibrary.MakeVector` 0.0 (`KismetMathLibrary.RandomFloatInRange` 20.0 -20.0) 50.0)) (struct) (0.2 0.2 0.2)) "AlwaysSpawn" "OverrideRootScale" null null)))

(fn `UserConstructionScript`)